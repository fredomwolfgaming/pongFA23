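; An unfinished AI paddle Blueprint, apparently meant to act on a ball actor.
; BeginPlay looks up the Bp_ball actor, but the result never feeds into the movement.
; Tick calls MoveComponentTo on the Cube component every frame with a one-second duration and no target wired, so no tracking logic exists yet.
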(event EventBeginPlay
  (|CallParentFunction)
  (bind _returnvalue (Actor|GetActorOfClass "/Game/bp_ball.bp_ball_C")))

(event Collision|EventActorBeginOverlap
  (params (OtherActor :type Actor%20Object%20Reference))
  (|CallParentFunction OtherActor) ; This node is disabled and will not be called.\nDrag off pins to build functionality.
)

(event EventTick
  (params (DeltaSeconds :type Float%20%28single-precision%29))
  (|CallParentFunction DeltaSeconds)
  (Components|MoveComponentTo (Variables|Default|GetCube) (Math|Vector|MakeVector 0.0 0.0 0.0) "0, 0, 0" false false 1.0 false))

(fn ConstructionScript
  (|CallParentFunction))