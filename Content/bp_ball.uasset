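; Pong-style ball that launches toward the player at a random sideways angle and feeds AI tracking when the player hits it.
; BeginPlay applies the starting impulse and caches the first player paddle.
; A blocking hit from that paddle runs SendAiTracker, spawning an invisible ball at fixed height above the play position.
; It estimates direction from positions sampled across a short delay, then launches the tracker along that vector with a large impulse.
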(event EventBeginPlay
  (bind _returnvalue (Math|Random|RandomFloatinRange 0.01 0.99))
  (bind _inital_inpulse_speed_multiplier (Variables|Default|Getinital%20inpulse%20speed%20multiplier))
  ;[1 1 1] random percentage of 90* angle, but not entirely one vector. random to decide if reflected on y axis. only get once. used as x vector
  (if (Math|Random|RandomBool)
    (Variables|Default|SetX%20inpulse%20vector%20percentage (* -1 _returnvalue))
    (else
      (Variables|Default|SetX%20inpulse%20vector%20percentage _returnvalue)))
  ;[1 1 1] inpulse addition. standard L/R speed.
  (Physics|AddImpulse (Variables|Default|GetSphere) (Math|Vector|MakeVector (* (Variables|Default|GetX%20inpulse%20vector%20percentage) _inital_inpulse_speed_multiplier) (* -1.0 _inital_inpulse_speed_multiplier) 0.0) "None" false)
  (bind _outactors (Actor|GetAllActorsOfClass "/Game/bp_paddle_Player.bp_paddle_Player_C"))
  (Variables|Default|Setplayer (Utilities|Array|Get(acopy) _outactors)))

(event Collision|EventActorBeginOverlap
  (params (OtherActor :type Actor%20Object%20Reference)))

(event Collision|EventHit
  (params (MyComp :type Primitive%20Component%20Object%20Reference) (Other :type Actor%20Object%20Reference) (OtherComp :type Primitive%20Component%20Object%20Reference) (bSelfMoved :type Boolean) (HitLocation :type Vector :default "0, 0, 0") (HitNormal :type Vector :default "0, 0, 0") (NormalImpulse :type Vector :default "0, 0, 0") (Hit :type Hit%20Result%20Structure%20%28by%20ref%29))
  (if (.bBlockingHit (Collision|BreakHitResult Hit))
    (if (== Other (Variables|Default|Getplayer))
      (|SendAiTracker))))

(fn ConstructionScript)